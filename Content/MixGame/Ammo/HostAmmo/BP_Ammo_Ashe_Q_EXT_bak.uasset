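; Ammo actor, apparently a backup of an Ashe Q ability variant, that damages non-friendly creatures it touches.
; Its Box overlap casts the other actor to MixCreature and skips friendly heroes, the player's own hero and friendly Batman types.
; Any other creature gets its name printed as debug output, is set as the target, and receives damage through CauseDamage.
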(event OnComponentBeginOverlap(Box)
  (params (OverlappedComponent :type Primitive%20Component%20Object%20Reference) (OtherActor :type Actor%20Object%20Reference) (OtherComp :type Primitive%20Component%20Object%20Reference) (OtherBodyIndex :type Integer) (bFromSweep :type Boolean) (SweepResult :type Hit%20Result%20Structure%20%28by%20ref%29))
  (bind _asmix_creature (Utilities|Casting|CastToMixCreature OtherActor))
  (if (not (Math|Boolean|ORBoolean (== (Variables|/Script/MyGame.MixCreature|GetCreatureType _asmix_creature) "(TagName=\"Creature.Type.Hero.Friend\")") (== (Variables|/Script/MyGame.MixCreature|GetCreatureType _asmix_creature) "(TagName=\"Creature.Type.Hero.Self\")") (== (Variables|/Script/MyGame.MixCreature|GetCreatureType _asmix_creature) "(TagName=\"Creature.Type.Batman.Friend\")")))
    (Development|PrintString (Utilities|GetDisplayName _asmix_creature) true true "(R=0.894444,G=1.000000,B=0.892754,A=1.000000)")
    (Class|MixRangedAmmo|SetTarget _asmix_creature)
    (Class|MixRangedAmmo|CauseDamage)))

(event EventBeginPlay)

(event Collision|EventActorBeginOverlap
  (params (OtherActor :type Actor%20Object%20Reference)))

(event EventTick
  (params (DeltaSeconds :type Float%20%28single-precision%29)))

(fn ConstructionScript)