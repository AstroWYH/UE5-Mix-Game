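; Ability Blueprint for the hero Ashe's Q, which fires from the bow and places a second ammo actor at the mouse location.
; PerformAbility prints a debug message and plays the Q montage on the Hero.
; OnMontageNotify spawns BP_Ammo_Ashe_Q at the bow emitter socket and BP_Ammo_Ashe_Q_EXT at the passed mouse location, setting the Hero as shooter only on the latter.
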(event EventBeginPlay)

(event Collision|EventActorBeginOverlap
  (params (OtherActor :type Actor%20Object%20Reference)))

(event EventTick
  (params (DeltaSeconds :type Float%20%28single-precision%29)))

(event EventPerformAbility
  (Development|PrintString "我按了艾希的Q")
  (Animation|PlayAnimMontage (Variables|Default|GetHero) "/Game/MixGame/Character/Host/Animations/Ashe_Montage_Q.Ashe_Montage_Q" 1.0 "None"))

(event EventOnMontageNotify
  (params (MouseLocation :type Vector%20%28by%20ref%29 :default "0, 0, 0"))
  (Game|SpawnActorfromClass "/Game/MixGame/Ammo/HostAmmo/BP_Ammo_Ashe_Q.BP_Ammo_Ashe_Q_C" (Transformation|GetSocketTransform (Variables|/Script/Engine.Character|GetMesh (Variables|Default|GetHero)) "BowEmitterSocket" "RTS_World") "AdjustIfPossibleButAlwaysSpawn" "MultiplyWithRoot" 0 0)
  (bind _returnvalue (Game|SpawnActorfromClass "/Game/MixGame/Ammo/HostAmmo/BP_Ammo_Ashe_Q_EXT.BP_Ammo_Ashe_Q_EXT_C" (Math|Transform|MakeTransform MouseLocation "0, 0, 0" "1.000000,1.000000,1.000000") "AdjustIfPossibleButAlwaysSpawn" "MultiplyWithRoot" 0 0))
  (Class|MixRangedAmmo|SetShooter _returnvalue (Variables|Default|GetHero)))

(fn ConstructionScript)