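; BP_HeroController is the hero's controller Blueprint, whose input and click-to-move logic has been moved to C++.
; The remaining graphs are unconnected leftovers: Enhanced Input mapping and look input, plus a right-click move prototype.
; That prototype traces from the deprojected cursor to a ground point at fixed height and steers the hero toward a target while setting IsPatrol.
; Tick and the construction script are empty.
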(event Input|EnhancedActionEvents|EnhancedInputActionHostInput_Look
  (params (ActionValue :type Vector%202D%20Structure) (ElapsedSeconds :type Float%20%28double-precision%29) (TriggeredSeconds :type Float%20%28double-precision%29) (InputAction :type Input%20Action%20Object%20Reference :default "/Game/MixGame/Character/Host/Input/HostInput_Look.HostInput_Look"))
  ;[1 0 0.3799] 增强输入在蓝图的用法
  ;;[1 1 1] 这步在Cpp里做了
)

(event EventTick
  (params (DeltaSeconds :type Float%20%28single-precision%29))
  ;[1 0.2977 0.5418] 挪至C++ 主角走到右键点击的位置
)

(event Input|MouseEvents|RightMouseButton
  (params (Key :type Key%20Structure :default "None"))
  ;[1 0.5639 0] 挪至C++ 鼠标屏幕位置转换为3D空间位置
)

(fn ConstructionScript)