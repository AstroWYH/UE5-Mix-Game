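; Host character Blueprint for MixGame, whose graphs hold no live logic.
; A note says the left-click attack montage moved to C++, with a montage notify reaching the anim Blueprint, which calls spawn.
; HostAttackSpawn is an empty event here.
; Disconnected leftover nodes show an earlier montage attack, a HostArrow spawn at the bow socket, and debug cylinder and trace experiments.
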(event EventBeginPlay)

(event Collision|EventActorBeginOverlap
  (params (OtherActor :type Actor%20Object%20Reference)))

(event EventTick
  (params (DeltaSeconds :type Float%20%28single-precision%29)))

(event Custom|HostAttackSpawn
  ;[1 1 1] 攻击蒙太奇通知动画蓝图 ，动画蓝图调用spawn
)

(event EventTick
  (params (DeltaSeconds :type Float%20%28single-precision%29)))

(event Input|MouseEvents|LeftMouseButton
  (params (Key :type Key%20Structure :default "None")))

(event Input|MouseEvents|LeftMouseButton
  (params (Key :type Key%20Structure :default "None"))
  ;[1 1 1] 挪至C++ 左键攻击播放蒙太奇
)

(fn ConstructionScript)