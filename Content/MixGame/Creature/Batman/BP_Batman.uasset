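; BP_Batman is a creature character Blueprint whose attack logic is currently disconnected, so none of it runs.
; The montage and spawn attack events and BeginPlay are empty.
; Orphaned nodes hold an IsAttack-gated montage with a delayed reset, a BatmanAmmo spawn at LaunchPoint, and a debug print of CharacterAttackComponent's name.
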(event EventBeginPlay)

(event Collision|EventActorBeginOverlap
  (params (OtherActor :type Actor%20Object%20Reference)))

(event EventTick
  (params (DeltaSeconds :type Float%20%28single-precision%29)))

(event Custom|BatmanAttackMontage
  ;[0.8914 0.4114 1] Comment
)

(event Custom|BatmanAttackSpawn
  ;[0.8914 0.4114 1] Comment
)

(event EventBeginPlay)

(fn ConstructionScript)