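; BP_BatmanController is the AI controller for the Batman creature.
; On BeginPlay it runs the BT_Batman_Bak behavior tree, sets the BB_Batman blackboard and calls BpPostBeginPlay.
; The perception update event is empty.
; Logic for gathering tagged patrol points, initializing the patrol index and writing hero detection to the blackboard is present but disconnected, so it never runs.
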(event OnTargetPerceptionUpdated(AIPerception)
  (params (Actor :type Actor%20Object%20Reference) (Stimulus :type AI%20Stimulus%20Structure))
  ;[0.8439 0.3046 1] AI perception视野检测，设置Isdetecthero
)

(event EventBeginPlay
  ;[1 1 1] 只有这在run
  (AI|RunBehaviorTree "/Game/MixGame/Creature/Batmans/AI/BT_Batman_Bak.BT_Batman_Bak")
  (Class|AIController|UseBlackboard "/Game/MixGame/Creature/Batmans/AI/BB_Batman.BB_Batman")
  (Class|MixAIController|BpPostBeginPlay))

(fn ConstructionScript)