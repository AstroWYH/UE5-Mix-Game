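; Player controller for the host hero, whose live Blueprint logic consists only of two debug keys that swap control of that hero.
; The first key spawns an AI controller to possess the host hero and focus the second spawned hero; the other has this controller possess the host again.
; Enhanced Input setup and right-click-to-move (cursor trace, walk to point) are noted as moved to C++, leaving their Blueprint nodes disconnected.
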(event Input|EnhancedActionEvents|EnhancedInputActionHostInput_Look
  (params (ActionValue :type Vector%202D%20Structure) (ElapsedSeconds :type Float%20%28double-precision%29) (TriggeredSeconds :type Float%20%28double-precision%29) (InputAction :type Input%20Action%20Object%20Reference :default "/Game/MixGame/Creature/Host/Input/HostInput_Look.HostInput_Look"))
  ;[1 0 0.3799] 增强输入在蓝图的用法
  ;;[1 1 1] 这步在Cpp里做了
)

(event Input|KeyboardEvents|DebugKey1
  (params (Key :type Key%20Structure :default "None") (ActionValue :type Input%20Action%20Value%20Structure))
  (bind _returnvalue (Subsystems|GetMixLevelSubsystem))
  (:Pressed
    (bind _returnvalue_2 (Game|SpawnActorfromClass "/Script/AIModule.AIController" (Math|Transform|MakeTransform "0, 0, 0" "0, 0, 0" "1.000000,1.000000,1.000000") "AlwaysSpawn" "MultiplyWithRoot" 0 0))
    (Pawn|Possess _returnvalue_2 (Class|MixLevelSubsystem|GetHostHero _returnvalue))
    (AI|SetFocus _returnvalue_2 (Utilities|Array|Get(acopy) (Class|MixLevelSubsystem|GetSpawnedHeros _returnvalue) 1))))

(event Input|KeyboardEvents|DebugKey2
  (params (Key :type Key%20Structure :default "None") (ActionValue :type Input%20Action%20Value%20Structure))
  (:Pressed
    (Pawn|Possess self (Class|MixLevelSubsystem|GetHostHero (Subsystems|GetMixLevelSubsystem)))))

(event EventTick
  (params (DeltaSeconds :type Float%20%28single-precision%29))
  ;[1 0.2977 0.5418] 挪至C++ 主角走到右键点击的位置
)

(event Input|MouseEvents|RightMouseButton
  (params (Key :type Key%20Structure))
  ;[1 0.5639 0] 挪至C++ 鼠标屏幕位置转换为3D空间位置
)

(fn ConstructionScript)